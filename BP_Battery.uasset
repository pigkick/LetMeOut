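; BP_Battery is a pickup that adds battery charge to the player character when they interact with it.
; Its PlayerDetecter overlap enables input, shows the W_Interraction_Battery prompt widget and opens a gate; leaving the overlap reverses all three.
; The IA_Interract input only passes the open gate, then calls IncreaseBattery on the player, plays a 2D sound and destroys the actor.
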(event `EnhancedInput|/Game/ThirdPerson/Input/Actions/IA_Interract`
  (params (ActionValue :type Boolean) (ElapsedSeconds :type "Float (double-precision)") (TriggeredSeconds :type "Float (double-precision)") (InputAction :type "InputAction Object Reference" :default "/Game/ThirdPerson/Input/Actions/IA_Interract.IA_Interract"))
  (:`Started`
    (`/Engine/EditorBlueprintResources/StandardMacros.Gate` true :!label _label
      (:`Exit`
        (bind _asbp_player_character (cast `/Game/ThirdPerson/Blueprints/BP_PlayerCharacter` (`GameplayStatics.GetPlayerCharacter` 0)))
        (`/Game/ThirdPerson/Blueprints/BP_PlayerCharacter.IncreaseBattery` _asbp_player_character 20.0)
        (`GameplayStatics.PlaySound2D` "/Game/StarterContent/Audio/paper-collect-2-186599.paper-collect-2-186599" 1.0 1.0 0.0 null null)
        (`self.K2_DestroyActor`)))))

(event `self.Player Detecter.OnComponentBeginOverlap`
  (params (OverlappedComponent :type "PrimitiveComponent Object Reference") (OtherActor :type "Actor Object Reference") (OtherComp :type "PrimitiveComponent Object Reference") (OtherBodyIndex :type Integer) (bFromSweep :type Boolean) (SweepResult :type "HitResult Structure (by ref)"))
  (cast `/Game/ThirdPerson/Blueprints/BP_PlayerCharacter` OtherActor)
  (`self.EnableInput` (`GameplayStatics.GetPlayerController` 0))
  ;[1 1 1] Create interraction
  (bind _returnvalue (`|CreateWidget` "/Game/ThirdPerson/UI/W_Interraction_Battery.W_Interraction_Battery_C"))
  (bind _output_get (set `self.W_Interraction_Battery` _returnvalue))
  (`UserWidget.AddToViewport` _output_get 0)
  (goto _label :!via `Open`))

(event `self.Player Detecter.OnComponentEndOverlap`
  (params (OverlappedComponent :type "PrimitiveComponent Object Reference") (OtherActor :type "Actor Object Reference") (OtherComp :type "PrimitiveComponent Object Reference") (OtherBodyIndex :type Integer))
  (cast `/Game/ThirdPerson/Blueprints/BP_PlayerCharacter` OtherActor)
  (`self.DisableInput` (`GameplayStatics.GetPlayerController` 0))
  (bind _w_interraction_battery (`self.W_Interraction_Battery`)
    (:`then`
      (`Widget.RemoveFromParent` _w_interraction_battery)
      (set `self.W_Interraction_Battery` null)
      (goto _label :!via `Close`))
    (:`else`
      (goto _label :!via `Close`))))

(fn `UserConstructionScript`)